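; BP_FloorTile is an infinite runner track segment that randomizes its contents and chains to the next tile.
; Its construction script spawns either a blocker at one of three spawn points or coins scattered within CoinArea.
; When the player overlaps EndTrigger, it asks the GameMode to add a tile, then destroys itself after a delay.
; Wall hits use a normal-versus-forward dot product to trigger controller Death only on head-on impacts.
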(event OnComponentBeginOverlap(EndTrigger)
  (params (OverlappedComponent :type Primitive%20Component%20Object%20Reference) (OtherActor :type Actor%20Object%20Reference) (OtherComp :type Primitive%20Component%20Object%20Reference) (OtherBodyIndex :type Integer) (bFromSweep :type Boolean) (SweepResult :type Hit%20Result%20Structure%20%28by%20ref%29))
  (if (== OtherActor (Variables|Default|GetRefThirdPersonCharacter))
    (Default|AddFloorTile (Variables|Default|GetRefThirdPersonGameMode))
    (Utilities|FlowControl|Delay 2.0)
    (Actor|DestroyActor)))

(event OnComponentHit(Wall_2)
  (params (HitComponent :type Primitive%20Component%20Object%20Reference) (OtherActor :type Actor%20Object%20Reference) (OtherComp :type Primitive%20Component%20Object%20Reference) (NormalImpulse :type Vector :default "0, 0, 0") (Hit :type Hit%20Result%20Structure%20%28by%20ref%29))
  (bind _asthird_person_character (Utilities|Casting|CastToThirdPersonCharacter OtherActor))
  (bind _asrun_player_controller (Utilities|Casting|CastToRunPlayerController (Pawn|GetController _asthird_person_character)))
  (if (Math|Float|NearlyEqual(Float) (Math|Vector|DotProduct (.normal Hit) (Transformation|GetActorForwardVector _asthird_person_character)) 1.0 0.01)
    (Default|Death _asrun_player_controller)))

(event OnComponentHit(Wall_1)
  (params (HitComponent :type Primitive%20Component%20Object%20Reference) (OtherActor :type Actor%20Object%20Reference) (OtherComp :type Primitive%20Component%20Object%20Reference) (NormalImpulse :type Vector :default "0, 0, 0") (Hit :type Hit%20Result%20Structure%20%28by%20ref%29))
  (bind _asthird_person_character (Utilities|Casting|CastToThirdPersonCharacter OtherActor))
  (bind _asrun_player_controller (Utilities|Casting|CastToRunPlayerController (Pawn|GetController _asthird_person_character)))
  (if (Math|Float|NearlyEqual(Float) (Math|Vector|DotProduct (.normal Hit) (Transformation|GetActorForwardVector _asthird_person_character)) 1.0 0.01)
    (Default|Death _asrun_player_controller)))

(event EventBeginPlay
  ;[1 1 1] Getting Ref. on BeginPlay of the Game
  (bind _asthird_person_character (Utilities|Casting|CastToThirdPersonCharacter (Game|Player|GetPlayerPawn 0)))
  (Variables|Default|SetRefThirdPersonCharacter _asthird_person_character)
  (bind _asthird_person_game_mode (Utilities|Casting|CastToThirdPersonGameMode (Game|GetGameMode)))
  (Variables|Default|SetRefThirdPersonGameMode _asthird_person_game_mode))

(fn ConstructionScript
  (CallFunction|SetSpawnPoint)
  (switch int (Math|Random|RandomIntegerinRange 0 1)
    (:Default
      (CallFunction|AddBlocker :!label _label))
    (:0
      (goto _label))
    (:1
      (CallFunction|SpawnCoin))))

(fn GetFloorTransform
  (return (Transformation|GetWorldTransform (Variables|Default|GetAttachPoint))))

(fn SetSpawnPoint
  (Variables|Default|SetSpawnPoints (Utilities|Array|MakeArray (Transformation|GetRelativeTransform (Variables|Default|GetSpawnPoint)) (Transformation|GetRelativeTransform (Variables|Default|GetSpawnPointL)) (Transformation|GetRelativeTransform (Variables|Default|GetSpawnPointR)))))

(fn AddBlocker
  (bind _spawnpoints (Variables|Default|GetSpawnPoints))
  (AddComponent|AddChildActorComponent false (Utilities|Array|Get(acopy) _spawnpoints (Math|Random|RandomIntegerinRange 0 (Utilities|Array|LastIndex _spawnpoints)))))

(fn SpawnCoin
  (bind _coinarea (Variables|Default|GetCoinArea))
  (for _index (range 0 5)
    (AddComponent|AddChildActorComponent false (Math|Conversions|ToTransform(Vector) (Math|Random|RandomPointinBoundingBox (Variables|/Script/Engine.SceneComponent|GetRelativeLocation _coinarea) (Variables|/Script/Engine.BoxComponent|GetBoxExtent _coinarea))))))