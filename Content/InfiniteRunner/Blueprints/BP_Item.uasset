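; BP_Item is a coin pickup for the infinite runner game.
; On BeginPlay it caches the player's ThirdPersonCharacter and RunPlayerController.
; When that character overlaps the Coin component, it calls AddCoin on the controller, plays a sound at its location and destroys itself.
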(event OnComponentBeginOverlap(Coin)
  (params (OverlappedComponent :type Primitive%20Component%20Object%20Reference) (OtherActor :type Actor%20Object%20Reference) (OtherComp :type Primitive%20Component%20Object%20Reference) (OtherBodyIndex :type Integer) (bFromSweep :type Boolean) (SweepResult :type Hit%20Result%20Structure%20%28by%20ref%29))
  (if (== OtherActor (Variables|Default|GetRefToThirdPerson))
    (Default|AddCoin (Variables|Default|GetRefToRunPlayerController))
    (Audio|PlaySoundatLocation 0 (Transformation|GetActorLocation) "0, 0, 0" 1.0 1.0 0.0 0 0 0)
    (Actor|DestroyActor)))

(event EventBeginPlay
  (bind _asthird_person_character (Utilities|Casting|CastToThirdPersonCharacter (Game|Player|GetPlayerPawn 0)))
  (Variables|Default|SetRefToThirdPerson _asthird_person_character)
  (bind _asrun_player_controller (Utilities|Casting|CastToRunPlayerController (Game|GetPlayerController 0)))
  (Variables|Default|SetRefToRunPlayerController _asrun_player_controller))

(event Collision|EventActorBeginOverlap
  (params (OtherActor :type Actor%20Object%20Reference)))

(event EventTick
  (params (DeltaSeconds :type Float%20%28single-precision%29)))

(fn ConstructionScript)